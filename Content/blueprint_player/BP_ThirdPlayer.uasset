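; BP_ThirdPlayer is a player Blueprint with axis-driven movement, mouse-based facing and a fire action.
; Each Tick, the mesh turns along the vector from viewport center to cursor, used directly as a world-space direction without a trace.
; Movement axes follow vectors derived from control rotation.
; Fire spawns an explosion emitter, 2D sound and an actor, placing emitter and actor at a scene component's location.
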(event EventBeginPlay
  (bind _asbp_playercontroll (Utilities|Casting|CastTobp_playercontroll (Pawn|GetController)))
  (Variables|Default|Setplayercontroller _asbp_playercontroll))

(event EventTick
  (params (DeltaSeconds :type Float%20%28single-precision%29))
  (bind _returnvalue (Viewport|GetViewportSize))
  (bind _returnvalue_2 (Class|WidgetLayoutLibrary|GetMousePositiononViewport))
  (bind _output_get (Variables|Default|Setdirection (Math|Vector|MakeVector (- (.x _returnvalue_2) (/ (.x _returnvalue) 2.0)) (- (.y _returnvalue_2) (/ (.y _returnvalue) 2.0)) 0.0)))
  (Transformation|SetWorldRotation (Variables|Character|GetMesh) (Math|Conversions|RotationFromXVector _output_get) false false))

(event Input|ActionEvents|InputActionfire
  (params (Key :type Key%20Structure :default "None"))
  (bind _scene (Variables|Default|GetScene))
  (bind _returnvalue (Transformation|GetWorldLocation _scene))
  (:Pressed
    (Effects|SpawnEmitteratLocation "/Game/StarterContent/Particles/P_Explosion.P_Explosion" _returnvalue)
    (Audio|SpawnSound2D "/Game/StarterContent/Audio/Explosion02.Explosion02" 1.0 1.0 0.0 0)
    (Game|SpawnActorfromClass "/Game/blueprint_player/bp_bullet.bp_bullet_C" (Math|Transform|MakeTransform _returnvalue "0, 0, 0" "1.000000,1.000000,1.000000") "Undefined" "MultiplyWithRoot" 0 0)))

(event Input|AxisEvents|InputAxisXvector
  (params (AxisValue :type Float%20%28single-precision%29))
  (Pawn|Input|AddMovementInput (Math|Vector|GetRightVector (Math|Rotator|MakeRotator 0.0 (.pitch (Pawn|GetControlRotation :!class /Script/Engine.Pawn)) 0.0)) AxisValue false))

(event Input|AxisEvents|InputAxisYvector
  (params (AxisValue :type Float%20%28single-precision%29))
  (Pawn|Input|AddMovementInput (Math|Vector|GetForwardVector (Math|Rotator|MakeRotator 0.0 0.0 (.yaw (Pawn|GetControlRotation :!class /Script/Engine.Pawn)))) AxisValue false))

(fn ConstructionScript)