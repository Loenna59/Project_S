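; BP_Boss is a boss character Blueprint that holds two helper functions, with no event logic in the file.
; UpdateWalkSpeed sets the CharacterMovement max walk speed and prints the new value.
; LookAt is a stub that only prints whether the given player reference is valid, without rotating the boss, and an unconnected location subtraction is left in the file.
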(fn ConstructionScript)

(fn UpdateWalkSpeed
  (params (NewWalkSpeed :type Float%20%28double-precision%29))
  (bind _output_get (Variables|/Script/Engine.CharacterMovementComponent|SetMaxWalkSpeed (Variables|Character|GetCharacterMovement) NewWalkSpeed))
  (Development|PrintString (Utilities|String|ToString(Float) _output_get)))

(fn Lookat
  (params (Player :type Actor%20Object%20Reference))
  (Utilities|IsValid Player
    (:Is%20Valid
      (Development|PrintString "valid"))
    (:Is%20Not%20Valid
      (Development|PrintString "invalid"))))