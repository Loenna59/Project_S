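; BP_FireBall is a fireball projectile that damages BP_Player on contact.
; Each Tick it moves with a sweep along Direction at Speed, both settable through setter functions.
; Overlapping the player calls Damaged, then the custom Destroy event removes the actor.
; A five-second Destroy timer is re-set every Tick, so it keeps restarting instead of limiting lifetime.
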(event OnComponentBeginOverlap(Collision)
  (params (OverlappedComponent :type Primitive%20Component%20Object%20Reference) (OtherActor :type Actor%20Object%20Reference) (OtherComp :type Primitive%20Component%20Object%20Reference) (OtherBodyIndex :type Integer) (bFromSweep :type Boolean) (SweepResult :type Hit%20Result%20Structure%20%28by%20ref%29))
  (bind _asbp_player (Utilities|Casting|CastToBP_Player OtherActor))
  (Default|Damaged _asbp_player (Variables|Default|GetDamage))
  (CallFunction|Destroy))

(event Custom|Destroy
  (Actor|DestroyActor)
  (Utilities|Time|ClearandInvalidateTimerbyHandle (Variables|Default|GetLifeTimer)))

(event EventTick
  (params (DeltaSeconds :type Float%20%28single-precision%29))
  (Transformation|SetActorLocation (+ (Transformation|GetActorLocation) (* DeltaSeconds (* (Variables|Default|GetSpeed) (Variables|Default|GetDirection)))) true false)
  (bind _returnvalue (Utilities|Time|SetTimerbyEvent (delegate Custom|Destroy) 5.0))
  (Variables|Default|SetLifeTimer _returnvalue))

(fn ConstructionScript)

(fn SetDirection
  (params (Direction :type Vector))
  (Variables|Default|SetDirection Direction))

(fn SetSpeed
  (params (NewSpeed :type Float%20%28double-precision%29))
  (Variables|Default|SetSpeed NewSpeed))