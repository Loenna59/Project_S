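; Item spawner actor that drops a pistol, armor and shoes pickup at random points within its box component.
; Register starts a separate, non-looping timer for each item at staggered delays and stores the handles so ClearAll can cancel them.
; Each timer event spawns its item within the central half-extent of the box and plays a lightning particle effect at that location through EmitPaticle.
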(event Custom|Register
  (bind _returnvalue (Utilities|Time|SetTimerbyEvent (delegate Custom|SpawnPistol) 1e+01))
  (Utilities|Array|Add (Variables|Default|GetTimeHandle) _returnvalue)
  (bind _returnvalue_2 (Utilities|Time|SetTimerbyEvent (delegate Custom|SpawnArmor) 15.0))
  (Utilities|Array|Add (Variables|Default|GetTimeHandle) _returnvalue_2)
  (bind _returnvalue_3 (Utilities|Time|SetTimerbyEvent (delegate Custom|SpawnShoes) 2e+01))
  (Utilities|Array|Add (Variables|Default|GetTimeHandle) _returnvalue_3))

(event Custom|SpawnPistol
  (bind _box (Variables|Default|GetBox))
  (bind (_origin _boxextent) (Collision|GetComponentBounds _box))
  (bind _returnvalue (Game|SpawnActorfromClass "/Game/Blueprints/BP_Pistol.BP_Pistol_C" (Math|Transform|MakeTransform (Math|Random|RandomPointinBoundingBox _origin (/ _boxextent 2.0)) "0, 0, 0" "1.000000,1.000000,1.000000") "Undefined" "MultiplyWithRoot" 0 0))
  (CallFunction|EmitPaticle (Transformation|GetActorLocation _returnvalue)))

(event Custom|SpawnArmor
  (bind _box (Variables|Default|GetBox))
  (bind (_origin _boxextent) (Collision|GetComponentBounds _box))
  (bind _returnvalue (Game|SpawnActorfromClass "/Game/TopDown/Blueprints/Bp_Armor.Bp_Armor_C" (Math|Transform|MakeTransform (Math|Random|RandomPointinBoundingBox _origin (/ _boxextent 2.0)) "0, 0, 0" "1.000000,1.000000,1.000000") "Undefined" "MultiplyWithRoot" 0 0))
  (CallFunction|EmitPaticle (Transformation|GetActorLocation _returnvalue)))

(event Custom|SpawnShoes
  (bind _box (Variables|Default|GetBox))
  (bind (_origin _boxextent) (Collision|GetComponentBounds _box))
  (bind _returnvalue (Game|SpawnActorfromClass "/Game/TopDown/Blueprints/Bp_Shoes.Bp_Shoes_C" (Math|Transform|MakeTransform (Math|Random|RandomPointinBoundingBox _origin (/ _boxextent 2.0)) "0, 0, 0" "1.000000,1.000000,1.000000") "Undefined" "MultiplyWithRoot" 0 0))
  (CallFunction|EmitPaticle (Transformation|GetActorLocation _returnvalue)))

(event Custom|ClearAll
  (for _array_element (Variables|Default|GetTimeHandle)
    (Utilities|Time|ClearandInvalidateTimerbyHandle _array_element)))

(fn ConstructionScript)

(fn EmitPaticle
  (params (Location :type Vector))
  (Effects|SpawnEmitteratLocation "/Game/FXVarietyPack/Particles/P_ky_lightning3.P_ky_lightning3" Location))