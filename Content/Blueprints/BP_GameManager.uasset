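; Game manager for a timed boss fight: spawns the Beholder boss, builds the UI and tracks Initialize, Playing, Complete, GameOver and TimeOver states.
; A player event triggers a one-time intro sequence, swapping in a stand-in boss, then starts the boss, countdown and item spawner.
; Boss completion plays a fade sequence into CompleteMap.
; Game over or timeout clears player, boss and items and shows the matching message.
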(event Custom|EventSequencePlay
  (bind _seuenceactor (Variables|SerializeField|GetSeuenceActor))
  (bind _sequenceplayer (Variables|/Script/LevelSequence.LevelSequenceActor|GetSequencePlayer _seuenceactor))
  (if (not (Variables|Default|GetIsPlayedSequence))
    (Variables|Default|SetIsPlayedSequence true)
    (EventDispatchers|BindEventtoOnFinished _sequenceplayer (delegate Custom|EventStart))
    (CallFunction|SwapBossVisiblity true)
    (Sequencer|Player|Play _sequenceplayer :!class /Script/MovieScene.MovieSceneSequencePlayer)
    (Input|DisableInput (Variables|Default|GetPlayer) (Game|GetPlayerController 0))))

(event Custom|EventStart
  (Input|EnableInput (Variables|Default|GetPlayer) (Game|GetPlayerController 0))
  (CallFunction|SwapBossVisiblity false)
  (Default|SetTimerText (Variables|Default|GetUI) (Variables|Default|GetRemainTime))
  (CallFunction|SetVisibleUI true)
  (Default|Start (Variables|Default|GetBoss))
  (Rendering|SetVisibility (Variables|/Game/TopDown/Blueprints/BP_TopDownCharacter.BP_TopDownCharacter_C|Gethealth%20Bar%20widget (Variables|Default|GetPlayer)) true false)
  (CallFunction|ChangeGameState "NewEnumerator1")
  (Default|Register (Variables|SerializeField|GetItemSpawner) (Variables|Constant|GetSpawnTimeArray)))

(event Custom|EventComplete
  (Rendering|SetVisibility (Variables|/Game/TopDown/Blueprints/BP_TopDownCharacter.BP_TopDownCharacter_C|Gethealth%20Bar%20widget (Variables|Default|GetPlayer)) false false)
  (CallFunction|ChangeGameState "NewEnumerator4")
  (Widget|SetVisibility (Variables|Default|GetUI) "Hidden")
  (bind _returnvalue (Sequencer|Player|CreateLevelSequencePlayer "/Game/LevelSequences/FadeSequence.FadeSequence"))
  (EventDispatchers|BindEventtoOnFinished _returnvalue (delegate Custom|EventFinish))
  (Sequencer|Player|Play _returnvalue :!class /Script/MovieScene.MovieSceneSequencePlayer))

(event Custom|EventGameOver
  (CallFunction|ChangeGameState "NewEnumerator2"))

(event Custom|EventFinish
  (Game|OpenLevel(byName) "CompleteMap"))

(event EventBeginPlay
  (CallFunction|ChangeGameState "NewEnumerator0")
  (CallFunction|CustructUI)
  (CallFunction|BindBoss (delegate Custom|EventComplete))
  (Variables|Default|SetRemainTime (Variables|Constant|GetTimeLimit))
  (CallFunction|BindPlayer (delegate Custom|EventSequencePlay) (delegate Custom|EventGameOver)))

(event EventTick
  (params (DeltaSeconds :type Float%20%28single-precision%29))
  (if (Utilities|Enum|Equal(Enum) (Variables|Default|GetState) "NewEnumerator1")
    (bind _output_get (Variables|Default|SetRemainTime (- (Variables|Default|GetRemainTime) DeltaSeconds)))
    (Default|SetTimerText (Variables|Default|GetUI) _output_get)
    (if (<= (Variables|Default|GetRemainTime) 0.0)
      (CallFunction|ChangeGameState "NewEnumerator3"))))

(fn ConstructionScript)

(fn CustructUI
  (bind _returnvalue (Game|ConstructObjectfromClass "/Game/Blueprints/WBP_UI.WBP_UI_C"))
  (bind _output_get (Variables|Default|SetUI _returnvalue))
  (CallFunction|SetVisibleUI false)
  (UserInterface|Viewport|AddtoViewport _output_get 0))

(fn BindBoss
  (params (CompleteEvent :type Delegate%20%28by%20ref%29))
  (bind _returnvalue (Game|SpawnActorfromClass "/Game/Blueprints/BP_Beholder.BP_Beholder_C" (Transformation|GetActorTransform (Variables|SerializeField|GetBossSpawner)) "Undefined" "MultiplyWithRoot" 0 0))
  (bind _output_get (Variables|Default|SetBoss _returnvalue))
  (Default|Initialize _output_get (EventDispatchers|CreateEvent (Variables|Default|GetUI) :!event SetHpUI) CompleteEvent))

(fn BindPlayer
  (params (StartEvent :type Delegate%20%28by%20ref%29) (GameOverEvent :type Delegate%20%28by%20ref%29))
  (bind _returnvalue (Actor|GetActorOfClass "/Game/Blueprints/BP_Player.BP_Player_C"))
  (bind _output_get (Variables|Default|SetPlayer _returnvalue))
  (bind _asbp_player (Utilities|Casting|CastToBP_Player _output_get))
  (Default|Initialize _asbp_player (Variables|Default|GetUI))
  (EventDispatchers|BindEventtoOnStartSequece _asbp_player StartEvent)
  (EventDispatchers|BindEventtoOnGameOver _asbp_player GameOverEvent))

(fn SetVisibleUI
  (params (Visible :type Boolean))
  (bind _ui (Variables|Default|GetUI))
  (Utilities|IsValid _ui
    (:Is%20Valid
      (if Visible
        (Widget|SetVisibility _ui "Visible")
        (else
          (Widget|SetVisibility _ui "Hidden"))))))

(fn SwapBossVisiblity
  (params (IsCopycat :type Boolean))
  (bind _returnvalue (Actor|GetActorOfClass "/Game/Blueprints/BP_Beholer_Sequence.BP_Beholer_Sequence_C"))
  (Utilities|IsValid _returnvalue
    (:Is%20Valid
      (Rendering|SetVisibility (Variables|/Game/Blueprints/BP_Beholer_Sequence.BP_Beholer_Sequence_C|GetSkeletalMesh _returnvalue) IsCopycat false)
      (Rendering|SetVisibility (Variables|/Script/Engine.Character|GetMesh (Variables|Default|GetBoss)) (not IsCopycat) false))))

(fn ChangeGameState
  (params (State :type E_GameState%20Enum :default "NewEnumerator0"))
  (bind _boss (Variables|Default|GetBoss))
  (bind _output_get (Variables|Default|SetState State))
  (switch Utilities|FlowControl|Switch|SwitchonE_GameState _output_get
    (:NewEnumerator4
      (Default|ClearAll (Variables|SerializeField|GetItemSpawner) :!label _label))
    (:NewEnumerator2
      (Default|ChangeState _boss "NewEnumerator0" :!label _label_2)
      (Default|ClearAll (Variables|Default|GetPlayer))
      (Default|Clear _boss)
      (if true
        (Default|ShowGameOver (Variables|Default|GetUI) (Utilities|String|SelectString "Game Over" "Time Over" (Utilities|Enum|Equal(Enum) (Variables|Default|GetState) "NewEnumerator2")))
        (goto _label)))
    (:NewEnumerator3
      (goto _label_2))))