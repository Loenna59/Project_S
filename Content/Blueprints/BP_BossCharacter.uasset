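; Boss character that patrols until it detects the player, then runs an attack pattern, with health and game-completion events for outside listeners.
; An enum state machine switches between Idle, Attack and Dead.
; Attack chains timers and rebinds the rotate-finished event: three jumps with fireball rings on landing, a rush, then a random laser or fireball spread.
; Damage skips the hit montage during lasers; death clears timers and delays destruction.
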(event Custom|Clear
  (Default|Clear (Variables|Default|GetLaserSpawnerComponent))
  (Utilities|Time|ClearandInvalidateTimerbyHandle (Variables|TimerHandle|GetDetectTimer))
  (Utilities|Time|ClearandInvalidateTimerbyHandle (Variables|TimerHandle|GetJumpTimer))
  (Utilities|Time|ClearandInvalidateTimerbyHandle (Variables|TimerHandle|GetRotateTimer))
  (Utilities|Time|ClearandInvalidateTimerbyHandle (Variables|TimerHandle|GetRushTimer))
  (Utilities|Time|ClearandInvalidateTimerbyHandle (Variables|TimerHandle|GetAttackDelayTimer))
  (bind _returnvalue (Utilities|Time|SetTimerbyEvent (delegate Custom|Destoy) 5.0))
  (Variables|TimerHandle|SetLifeTimer _returnvalue))

(event Custom|Destoy
  (Actor|DestroyActor)
  (Utilities|Time|ClearandInvalidateTimerbyHandle (Variables|TimerHandle|GetLifeTimer)))

(event EventTick
  (params (DeltaSeconds :type Float%20%28single-precision%29))
  (switch Utilities|FlowControl|Switch|SwitchonE_BossState (Variables|Default|GetCurrentState)
    (:NewEnumerator1
      (IdleState|TickIdleState DeltaSeconds))
    (:NewEnumerator2
      (AttackState|TickAttackState))))

(event Custom|EventShot
  (bind _delaytime (CallFunction|ShotBulletorFlame (stale Custom|ShotBulletForward _output_get)))
  (Utilities|Time|SetTimerbyEvent (delegate Custom|FinishAttack) _delaytime)
  (EventDispatchers|UnbindEventfromOnCompletedRotate (delegate Custom|ShotBulletForward)))

(event Custom|PlayJumpAndShot
  (Variables|AttackState|SetJumpCount 0)
  (bind _returnvalue (Utilities|Time|SetTimerbyEvent (delegate Custom|PlayJump) 1.0 true))
  (Variables|TimerHandle|SetJumpTimer _returnvalue)
  (CallFunction|PlayJump))

(event Custom|ShotBulletForward
  (bind _returnvalue (Utilities|Time|SetTimerbyEvent (delegate Custom|EventShot) 0.25))
  (Variables|TimerHandle|SetAttackDelayTimer _returnvalue)
  (bind _output_get (Variables|AttackState|SetIsPlayingLaserAttack (Math|Random|RandomBool)))
  (Variables|AttackState|SetIsPlayingBulletAttack (not _output_get)))

(event Custom|PlayJump
  (bind _jumpcount (Variables|AttackState|GetJumpCount))
  (Character|Jump)
  (if (Variables|AttackState|GetJumping)
    _
    (else
      (Variables|AttackState|SetJumping true)))
  (Math|Integer|IncrementInt _jumpcount
    (:%20%20
      (if (> _jumpcount 2)
        (Utilities|FlowControl|Sequence
          (:then_0
            (EventDispatchers|BindEventtoOnCompletedRotate (delegate Custom|RushEvent))
            (bind _returnvalue (Utilities|Time|SetTimerbyEvent (delegate Custom|RotateTarget) 1.0 false false 0.2))
            (Variables|TimerHandle|SetRotateTimer _returnvalue))
          (:then_1
            (Utilities|Time|ClearandInvalidateTimerbyHandle (Variables|TimerHandle|GetJumpTimer))))))))

(event Custom|RotateTarget
  (bind _returnvalue (Actor|GetActorOfClass "/Game/Blueprints/BP_Player.BP_Player_C"))
  (bind _value (Timeline|OnRotateCharacter Play)
    (:Update
      (Transformation|SetActorRotation (* (Math|Rotator|FindLookatRotation (Transformation|GetActorLocation) (Transformation|GetActorLocation _returnvalue)) _value)))
    (:Finished
      (Default|CallOnCompletedRotate))))

(event Custom|FinishAttack
  (Variables|AttackState|SetIsFinishAttackPattern true))

(event Custom|RushEvent
  (bind _duration (CallFunction|Rush (stale Custom|RotateTarget _returnvalue)))
  (bind _returnvalue (Utilities|Time|SetTimerbyEvent (delegate Custom|RotateTarget) _duration))
  (Variables|TimerHandle|SetRushTimer _returnvalue)
  (EventDispatchers|UnbindEventfromOnCompletedRotate (delegate Custom|RushEvent))
  (EventDispatchers|BindEventtoOnCompletedRotate (delegate Custom|ShotBulletForward)))

(event EventOnLanded
  (params (Hit :type Hit%20Result%20Structure%20%28by%20ref%29))
  ;[0.15 0.15 0.15 0.5] 땅에 닿는 순간 점프한 상태였다면 탄막을 발사
  (if (Variables|AttackState|GetJumping)
    (Audio|SpawnSoundatLocation "/Game/Sounds/footstep_grass_004.footstep_grass_004" (Transformation|GetActorLocation) "0, 0, 0" 1.0 1.0 0.0 0 0)
    (CallFunction|ShotBulletCircle)
    (if (Variables|AttackState|GetJumping)
      (Variables|AttackState|SetJumping false))))

(fn ConstructionScript)

(fn UpdateWalkSpeed
  (params (NewWalkSpeed :type Float%20%28double-precision%29))
  (Variables|/Script/Engine.CharacterMovementComponent|SetMaxWalkSpeed (Variables|Character|GetCharacterMovement) NewWalkSpeed))

(fn ShotBulletCircle
  (for _index (range 0 15)
    (bind _returnvalue (Game|SpawnActorfromClass "/Game/Blueprints/BP_FireBall.BP_FireBall_C" (Math|Transform|MakeTransform (Transformation|GetActorLocation) "0, 0, 0" "1.000000,1.000000,1.000000") "Undefined" "MultiplyWithRoot" 0 0))
    (Utilities|IsValid _returnvalue
      (:Is%20Valid
        (Default|SetSpeed _returnvalue (LocalVariables|GetBulletSpeed))
        (Default|SetDirection _returnvalue (Math|Vector|MakeVector (Math|Trig|Cos(Radians) (Math|Trig|DegreesToRadians (* _index (/ 3.6e+02 16.0)))) (Math|Trig|Sin(Radians) (Math|Trig|DegreesToRadians (* _index (/ 3.6e+02 16.0)))) 0.0))))))

(fn Initialize
  (params (UIEvent :type Delegate%20%28by%20ref%29) (CompleteEvent :type Delegate%20%28by%20ref%29))
  (EventDispatchers|BindEventtoOnUpdateHealth UIEvent)
  (EventDispatchers|BindEventtoOnCompleteGame CompleteEvent)
  (Variables|Stat|SetCurrentHp (Variables|Stat|GetBaseHp))
  (Components|Sphere|SetSphereRadius (Variables|Default|GetItemDropRadius) (Variables|Default|GetItemSpawnRadius) false)
  (Components|Sphere|SetSphereRadius (Variables|Default|GetDetectCollision) (Variables|IdleState|GetDetectCollisionRadius) true))

(fn Damaged
  (params (Damage :type Integer))
  (switch Utilities|FlowControl|Switch|SwitchonE_BossState (Variables|Default|GetCurrentState)
    (:NewEnumerator1
      (Animation|PlayAnimMontage "/Game/Blueprints/AM_Beholder_Damaged.AM_Beholder_Damaged" 2.0 "Damaged" :!label _label))
    (:NewEnumerator2
      (if (Variables|AttackState|GetIsPlayingLaserAttack)
        _
        (else
          (goto _label)))))
  (Audio|SpawnSoundatLocation "/Game/Free_Sounds_Pack/wav/Hit_Generic_2-1.Hit_Generic_2-1" (Transformation|GetActorLocation) "0, 0, 0" 1.0 1.0 0.0 0 0)
  (bind _output_get (Variables|Stat|SetCurrentHp (Math|Integer|Clamp(Integer) (- (Variables|Stat|GetCurrentHp) Damage) 0 (Variables|Stat|GetBaseHp))))
  (Default|CallOnUpdateHealth _output_get (Variables|Stat|GetBaseHp))
  (if (<= _output_get 0)
    (CallFunction|ChangeState "NewEnumerator3")))

(fn ChangeState
  (params (NewState :type E_BossState%20Enum :default "NewEnumerator0"))
  (if (Variables|Default|GetIsInitialState) ; initial state 일 경우 exit 상태로 플래그하고 스킵
    (Variables|Default|SetIsInitialState false)
    (Variables|Default|SetCurrentState NewState :!label _label)
    (Variables|Default|SetElapsedTimeInState 0.0)
    (switch Utilities|FlowControl|Switch|SwitchonE_BossState (Variables|Default|GetCurrentState)
      (:NewEnumerator1
        (IdleState|EnterIdleState))
      (:NewEnumerator2
        (AttackState|EnterAttackState))
      (:NewEnumerator3
        (CallFunction|EnterDeadState)))
    (elif (Utilities|Enum|NotEqual(Enum) NewState (Variables|Default|GetCurrentState))
      (switch Utilities|FlowControl|Switch|SwitchonE_BossState (Variables|Default|GetCurrentState)
        (:NewEnumerator0
          (goto _label))
        (:NewEnumerator1
          (IdleState|ExitIdleState)
          (goto _label))
        (:NewEnumerator2
          (AttackState|ExitAttackState)
          (goto _label))
        (:NewEnumerator3
          (goto _label))))))

(fn EnterIdleState
  (CallFunction|SetPatrolLocation)
  (EventDispatchers|BindEventtoOnDetected (EventDispatchers|CreateEvent :!event Detect)))

(fn TickIdleState
  (params (DeltaTime :type Float%20%28double-precision%29))
  (bind _returnvalue (Actor|GetActorOfClass "/Game/Blueprints/BP_Player.BP_Player_C"))
  (Utilities|IsValid _returnvalue
    (:Is%20Valid
      (if (Collision|IsOverlappingActor (Variables|Default|GetDetectCollision) _returnvalue :!class /Script/Engine.PrimitiveComponent)
        (CallFunction|Detect)
        (Variables|IdleState|SetCurrentMoveTime 0.0 :!label _label)
        (else
          (if (> (Variables|IdleState|GetCurrentMoveTime) (Variables|IdleState|GetMoveTime)) :!label _label_2
            (CallFunction|SetPatrolLocation)
            (goto _label)
            (else
              (Variables|IdleState|SetCurrentMoveTime (+ DeltaTime (Variables|IdleState|GetCurrentMoveTime))))))))
    (:Is%20Not%20Valid
      (goto _label_2))))

(fn ExitIdleState
  (Development|PrintString "Exit Idle State")
  (EventDispatchers|UnbindEventfromOnDetected (EventDispatchers|CreateEvent :!event Detect)))

(fn Detect
  (CallFunction|ChangeState "NewEnumerator2"))

(fn EnterAttackState
  (Utilities|Time|ClearandInvalidateTimerbyHandle (Variables|TimerHandle|GetDetectTimer))
  (CallFunction|PlayJumpandShot))

(fn ExitAttackState
  (Variables|AttackState|SetIsPlayingBulletAttack false)
  (Variables|AttackState|SetIsPlayingLaserAttack false)
  (Variables|AttackState|SetIsFinishAttackPattern false))

(fn TickAttackState
  (if (Variables|AttackState|GetIsFinishAttackPattern)
    (CallFunction|ChangeState "NewEnumerator1")))

(fn SetPatrolLocation
  (bind _output_get (Variables|IdleState|SetPatrolLocation (.RandomLocation (AI|Navigation|GetRandomReachablePointinRadius (Transformation|GetActorLocation) (Variables|IdleState|GetPatrolRadius) 0 0))))
  (AI|Navigation|SimpleMovetoLocation (Pawn|GetController) _output_get))

(fn Rush
  (params (Player :type Actor%20Object%20Reference))
  (Variables|/Script/Engine.CharacterMovementComponent|SetMaxWalkSpeed (Variables|Character|GetCharacterMovement) (Variables|Stat|GetRushSpeed))
  (AI|Navigation|SimpleMovetoLocation (Pawn|GetController) (Transformation|GetActorLocation Player))
  (return 2.0))

(fn ShotBulletorFlame
  (params (ExecuteLaser :type Boolean))
  (bind _returnvalue (Transformation|GetActorForwardVector))
  (bind _laserarrow (Variables|Default|GetLaserArrow))
  (bind _throwflameduration (Variables|AttackState|GetThrowFlameDuration))
  (if ExecuteLaser
    (bind _attach (Default|Spawn (Variables|Default|GetLaserSpawnerComponent) (Transformation|GetWorldLocation _laserarrow) (Transformation|GetWorldRotation _laserarrow) "(R=1.000000,G=0.000000,B=0.000000,A=1.000000)" _throwflameduration))
    (Audio|SpawnSoundAttached (LocalVariables|GetLaserSound) _attach "None" "0, 0, 0" "0, 0, 0" "KeepRelativeOffset" true 1.0 1.0 0.0 0 0)
    (Variables|Default|SetDelay%20Time _throwflameduration)
    (else
      (for _index (range 0 2)
        (bind _returnvalue_2 (Game|SpawnActorfromClass "/Game/Blueprints/BP_FireBall.BP_FireBall_C" (Math|Transform|MakeTransform (Transformation|GetActorLocation) "0, 0, 0" "1.000000,1.000000,1.000000") "Undefined" "MultiplyWithRoot" 0 0))
        (Utilities|IsValid _returnvalue_2
          (:Is%20Valid
            (Default|SetSpeed _returnvalue_2 (LocalVariables|GetBulletSpeed))
            (Default|SetDirection _returnvalue_2 (Math|Vector|RotateVector (Math|Vector|MakeVector (.x _returnvalue) (.y _returnvalue) 0.0) (Math|Rotator|MakeRotator 0.0 0.0 (* 3e+01 (- _index 1))))))))
      (Variables|Default|SetDelay%20Time (Variables|AttackState|GetShotBulletDuration))))
  (return (Variables|Default|GetDelay%20Time)))

(fn DropItem
  (bind _returnvalue (Transformation|GetActorLocation))
  (Game|SpawnActorfromClass "/Game/Blueprints/BP_Crate.BP_Crate_C" (Math|Transform|MakeTransform (.RandomLocation (AI|Navigation|GetRandomReachablePointinRadius (Math|Vector|MakeVector (.x _returnvalue) (.y _returnvalue) 0.0) (Variables|/Script/Engine.SphereComponent|GetSphereRadius (Variables|Default|GetItemDropRadius)) 0 0)) "0, 0, 0" "1.000000,1.000000,1.000000") "Undefined" "MultiplyWithRoot" 0 0))

(fn IsLaserAttack
  (return (Variables|AttackState|GetIsPlayingLaserAttack)))

(fn IsBulletAttack
  (return (Variables|AttackState|GetIsPlayingBulletAttack)))

(fn IsDead
  (switch Utilities|FlowControl|Switch|SwitchonE_BossState (Variables|Default|GetCurrentState)
    (:NewEnumerator0
      _)
    (:NewEnumerator1
      _)
    (:NewEnumerator2
      _)
    (:NewEnumerator3
      (return true)))
  (return false))

(fn GetDamaged
  (return (Variables|Default|GetIsDamaged)))

(fn EnterDeadState
  (CallFunction|Clear)
  (Default|CallOnCompleteGame))

(fn Start
  (Default|CallOnUpdateHealth (Variables|Stat|GetCurrentHp) (Variables|Stat|GetBaseHp))
  (CallFunction|ChangeState "NewEnumerator1"))