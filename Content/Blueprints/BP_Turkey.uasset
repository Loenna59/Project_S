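; BP_Turkey is an actor that homes in on the BP_TempPawn in the level.
; BeginPlay finds that pawn by class and stores it as Target.
; Each Tick moves the turkey straight toward Target at Speed, scaled by delta time, and turns it to face Target with a look-at rotation.
; Movement sets the transform directly, with no pathfinding or validity check on Target.
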(event EventBeginPlay
  (bind _returnvalue (Actor|GetActorOfClass "/Game/Blueprints/BP_TempPawn.BP_TempPawn_C"))
  (Variables|Default|SetTarget _returnvalue))

(event EventTick
  (params (DeltaSeconds :type Float%20%28single-precision%29))
  (bind _returnvalue (Transformation|GetActorLocation))
  (Transformation|SetActorLocationAndRotation (+ _returnvalue (* DeltaSeconds (* (Math|Vector|Normalize (- (Transformation|GetActorLocation (Variables|Default|GetTarget)) (Transformation|GetActorLocation))) (Variables|Default|GetSpeed)))) (Math|Rotator|FindLookatRotation _returnvalue (Transformation|GetActorLocation (Variables|Default|GetTarget)))))

(fn ConstructionScript)