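; Enemy actor Blueprint that chases the BP_ThirdPlayer character.
; Each Tick it looks up the player with GetActorOfClass, stores it as Target, and rotates to face it along the normalized direction vector.
; It then moves straight toward Target at Speed scaled by DeltaSeconds, without sweep, so movement ignores collision.
; A Finddirection function stores the same direction in Dimention, but Tick computes it inline instead.
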(event EventTick
  (params (DeltaSeconds :type Float%20%28single-precision%29))
  (bind _returnvalue (Actor|GetActorOfClass "/Game/blueprint_player/BP_ThirdPlayer.BP_ThirdPlayer_C"))
  (Variables|Default|Settarget _returnvalue)
  (Transformation|SetActorRotation (Math|Conversions|RotationFromXVector (Math|Vector|Normalize (- (Transformation|GetActorLocation (Variables|Default|Gettarget)) (Transformation|GetActorLocation)))))
  (Transformation|SetActorLocation (+ (Transformation|GetActorLocation) (* DeltaSeconds (* (Variables|Default|Getspeed) (Math|Vector|Normalize (- (Transformation|GetActorLocation (Variables|Default|Gettarget)) (Transformation|GetActorLocation)))))) false false))

(fn ConstructionScript)

(fn Finddirection
  (Variables|Default|Setdimention (Math|Vector|Normalize (- (Transformation|GetActorLocation (Variables|Default|Gettarget)) (Transformation|GetActorLocation)))))