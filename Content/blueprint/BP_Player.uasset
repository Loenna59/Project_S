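; BP_Player is a player Blueprint that moves from axis input and fires bullets.
; Each Tick offsets its location by Direction, Speed and delta time, without sweeping for collisions.
; The Horizental axis writes its value into all three Direction components, while the Vertical and Xvector axes are unimplemented.
; Pressing fire spawns a BP_Bullet at the player's location, and an unused right-vector movement node remains disconnected.
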(event EventTick
  (params (DeltaSeconds :type Float%20%28single-precision%29))
  ;[0.15 0.15 0.15 0.5] Comment
  (Transformation|SetActorLocation (+ (* DeltaSeconds (* (Variables|Default|Getspeed) (Variables|Default|Getdirection))) (Transformation|GetActorLocation)) false false))

(event Input|ActionEvents|InputActionfire
  (params (Key :type Key%20Structure :default "None"))
  ;[0.15 0.15 0.15 0.5] Comment
  (:Pressed
    (Game|SpawnActorfromClass "/Game/blueprint/BP_Bullet.BP_Bullet_C" (Math|Transform|MakeTransform (Transformation|GetActorLocation) "0, 0, 0" "1.000000,1.000000,1.000000") "Undefined" "MultiplyWithRoot" 0 0)))

(event Input|AxisEvents|InputAxisHorizental
  (params (AxisValue :type Float%20%28single-precision%29))
  ;[0.15 0.15 0.15 0.5] Comment
  (Variables|Default|Setdirection (Math|Vector|MakeVector AxisValue (stale Input|AxisEvents|InputAxisXvector AxisValue) (stale Input|AxisEvents|InputAxisVertical AxisValue))))

(event Input|AxisEvents|InputAxisVertical
  (params (AxisValue :type Float%20%28single-precision%29))
  ;[0.15 0.15 0.15 0.5] Comment
)

(event Input|AxisEvents|InputAxisXvector
  (params (AxisValue :type Float%20%28single-precision%29))
  ;[0.15 0.15 0.15 0.5] Comment
)

(fn ConstructionScript)