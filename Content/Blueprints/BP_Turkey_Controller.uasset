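; AI controller Blueprint for a turkey, built to track line of sight to a target through AI perception and a behavior tree.
; SetBlackboardValue writes the sight flag and player actor, and randomizes the flame trigger flag on each call.
; The behavior tree launch and the sensing logic with its lose-sight timer are disconnected, so the Possess and perception events currently do nothing.
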(event OnTargetPerceptionUpdated(AIPerception)
  (params (Actor :type Actor%20Object%20Reference) (Stimulus :type AI%20Stimulus%20Structure)))

(event Custom|SetEnemyTimer
  (CallFunction|SetBlackboardValue false))

(event EventPossess
  (params (PossessedPawn :type Pawn%20Object%20Reference)))

(fn ConstructionScript)

(fn SetBlackboardValue
  (params (BooleanValue :type Boolean) (ObjectValue :type Object%20Object%20Reference))
  (bind _blackboard (Variables|Default|GetBlackboard))
  (AI|Components|Blackboard|SetValueasBool _blackboard (Variables|Default|GetHasLineOfSight) BooleanValue)
  (AI|Components|Blackboard|SetValueasObject _blackboard (Variables|Default|GetPlayerActor) ObjectValue)
  (AI|Components|Blackboard|SetValueasBool _blackboard (Variables|Default|GetIsTriggerFlame) (Math|Random|RandomBool)))