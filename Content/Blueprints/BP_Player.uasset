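; Player Blueprint that configures camera distances and item attachment, and starts a sequence on entering trigger boxes.
; InteractCollision overlaps with a TriggerBox fire the OnStartSequece event dispatcher, while BeginPlay and Tick only call the parent.
; Setup functions define idle and hold camera arm lengths and assign RightArm as the attach slot.
; Equip snaps the given actor to RightArm's Attach socket and stores the attach result in Equipped.
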(event OnComponentBeginOverlap(InteractCollision)
  (params (OverlappedComponent :type Primitive%20Component%20Object%20Reference) (OtherActor :type Actor%20Object%20Reference) (OtherComp :type Primitive%20Component%20Object%20Reference) (OtherBodyIndex :type Integer) (bFromSweep :type Boolean) (SweepResult :type Hit%20Result%20Structure%20%28by%20ref%29))
  (Utilities|Casting|CastToTriggerBox OtherActor)
  (Default|CallOnStartSequece))

(event EventBeginPlay
  (|CallParentFunction))

(event EventTick
  (params (DeltaSeconds :type Float%20%28single-precision%29))
  (|CallParentFunction DeltaSeconds))

(fn ConstructionScript
  (|CallParentFunction))

(fn SetCameraArmLength
  (Variables|Default|SetIdleCameraArmLength 1.2e+03)
  (Variables|Default|SetHoldCameraArmLength 1.5e+03))

(fn SetAttachSlot
  (Variables|Default|SetRightArmSlot (Variables|Default|GetRightArm)))

(fn Equip
  (params (Actor :type Actor%20Object%20Reference))
  (bind _returnvalue (Transformation|AttachComponentToComponent Actor (Variables|Default|GetRightArm) "Attach" "SnapToTarget" "SnapToTarget" "SnapToTarget" true))
  (Variables|Default|SetEquipped _returnvalue))