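; BPP_Bush is a cherry bush that scatters BP_Cherry pickups around itself one time when Drop is called.
; BeginPlay fills a Degrees array with a few angles, each the loop index times a random offset.
; Drop uses cosine and sine to spawn a cherry at each angle, Distance away at the bush's height.
; It then marks the bush empty, disables Sphere collision and hides the Cherries component.
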(event EventBeginPlay
  (for _index (range 0 (Math|Random|RandomIntegerinRange 2 4))
    (Utilities|Array|Add (Variables|Default|GetDegrees) (* _index (Math|Random|RandomIntegerinRange -60 60)))))

(fn ConstructionScript)

(fn Drop
  (bind _returnvalue (Transformation|GetActorLocation))
  (if (not (Variables|Default|GetIsEmpty))
    (for _array_element (Variables|Default|GetDegrees)
      (Game|SpawnActorfromClass "/Game/Blueprints/BP_Cherry.BP_Cherry_C" (Math|Transform|MakeTransform (Math|Vector|MakeVector (+ (* (Math|Trig|Cos(Degrees) (Math|Conversions|ToFloat(Integer) _array_element)) (Variables|Default|GetDistance)) (.x _returnvalue)) (+ (* (Math|Trig|Sin(Degrees) (Math|Conversions|ToFloat(Integer) _array_element)) (Variables|Default|GetDistance)) (.y _returnvalue)) (.z _returnvalue)) "0, 0, 0" "1.000000,1.000000,1.000000") "Undefined" "MultiplyWithRoot" 0 0)
      (Variables|Default|SetIsEmpty true)
      (Collision|SetCollisionEnabled (Variables|Default|GetSphere) "NoCollision")
      (Rendering|SetVisibility (Variables|Default|GetCherries) false false))))